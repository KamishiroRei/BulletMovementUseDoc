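; BP_Bullet_Default is the demo's default bullet actor, driven by a BulletMovement component.
; It spawns pooled Niagara hit effects, aligned to the impact normal, on box hits and refractions, plus an end effect when destroyed.
; It destroys itself when movement stops and caches its owning demo character on BeginPlay.
; Unconnected nodes lay out the component's API, including forces, homing, refraction, return and trail setup, but never run.
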(event `self.ReceiveBeginPlay`
  (bind _asbp_demo_character (cast `/Game/DemoContent/Blueprint/BP_Demo_Character` (`self.GetOwner`)))
  (set `self.Character` _asbp_demo_character))

(event `self.BulletMovement.OnBulletRefracted`
  (params (Hit :type "HitResult Structure (by ref)") (Velocity :type "Vector Structure (by ref)"))
  (`self.SpawnHitVFX` Hit))

(event `self.BulletMovement.OnBulletStop`
  (params (Reason :type "E_BulletStopReason Enum" :default "Time"))
  (`self.K2_DestroyActor`)
  (switch `E_BulletStopReason` Reason))

(event `self.ReceiveDestroyed`
  (bind (_returnvalue_location _returnvalue_rotation _returnvalue_scale) (`KismetMathLibrary.BreakTransform` (`self.GetTransform`)))
  (`NiagaraFunctionLibrary.SpawnSystemAtLocation` (`self.EndVFX`) _returnvalue_location _returnvalue_rotation _returnvalue_scale true true "AutoRelease"))

(event `self.Box.OnComponentHit`
  (params (HitComponent :type "PrimitiveComponent Object Reference") (OtherActor :type "Actor Object Reference") (OtherComp :type "PrimitiveComponent Object Reference") (NormalImpulse :type "Vector Structure") (Hit :type "HitResult Structure (by ref)"))
  (`NiagaraFunctionLibrary.SpawnSystemAtLocation` (`self.HitVFX`) Hit_ImpactPoint (`KismetMathLibrary.Conv_VectorToRotator` Hit_ImpactNormal) (1.0 1.0 1.0) true true "AutoRelease"))

(fn `SpawnHitVFX`
  (params (Hit :type "HitResult Structure"))
  (`NiagaraFunctionLibrary.SpawnSystemAtLocation` (`self.HitVFX`) Hit_ImpactPoint (`KismetMathLibrary.Conv_VectorToRotator` Hit_ImpactNormal) (1.0 1.0 1.0) true true "AutoRelease"))

(fn `UserConstructionScript`)