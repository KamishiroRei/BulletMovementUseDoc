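; First-person demo character that moves, looks, jumps and switches between six bullet types on number keys 1-6.
; Bullet switches broadcast the selected index, and BeginPlay creates a bullet info widget bound to the character.
; A camera line trace each tick updates the look-at location and marker.
; Shooting only fires the OnUseItem dispatcher; SpawnBullet, not called here, spawns the selected type using its count, cone and randomness settings.
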(event `EnhancedInput|/Game/DemoContent/Blueprint/Input/IA_Look`
  (params (ActionValue :type "Vector2D Structure") (ElapsedSeconds :type "Float (double-precision)") (TriggeredSeconds :type "Float (double-precision)") (InputAction :type "InputAction Object Reference" :default "/Game/DemoContent/Blueprint/Input/IA_Look.IA_Look"))
  ; Character Input
  (:`Triggered`
    (`self.AddControllerYawInput` ActionValue_X)
    (`self.AddControllerPitchInput` ActionValue_Y)))

(event `EnhancedInput|/Game/DemoContent/Blueprint/Input/IA_Move`
  (params (ActionValue :type "Vector2D Structure") (ElapsedSeconds :type "Float (double-precision)") (TriggeredSeconds :type "Float (double-precision)") (InputAction :type "InputAction Object Reference" :default "/Game/DemoContent/Blueprint/Input/IA_Move.IA_Move"))
  ; Character Input
  (:`Triggered`
    (`self.AddMovementInput` (`self.GetActorRightVector`) ActionValue_X)
    (`self.AddMovementInput` (`self.GetActorForwardVector`) ActionValue_Y)))

(event `Key|One`
  (params (Key :type "Key Structure"))
  ; SetBullet
  (:`Pressed`
    (`self.BulletSwitch` 0)))

(event `self.ReceiveTick`
  (params (DeltaSeconds :type "Float (single-precision)"))
  ; Update LookAt
  (`self.UpdateLookAtLocation` DeltaSeconds))

(event `Key|Two`
  (params (Key :type "Key Structure"))
  ; SetBullet
  (:`Pressed`
    (`self.BulletSwitch` 1)))

(event `self.ReceiveBeginPlay`
  ; SpawnWidget
  (bind _returnvalue (`|CreateWidget` "/Game/DemoContent/Blueprint/UMG/UMG_Bullet_Info.UMG_Bullet_Info_C" (`GameplayStatics.GetPlayerController` 0) self))
  (`UserWidget.AddToViewport` _returnvalue 0))

(event `EnhancedInput|/Game/DemoContent/Blueprint/Input/IA_Jump`
  (params (ActionValue :type Boolean) (ElapsedSeconds :type "Float (double-precision)") (TriggeredSeconds :type "Float (double-precision)") (InputAction :type "InputAction Object Reference" :default "/Game/DemoContent/Blueprint/Input/IA_Jump.IA_Jump"))
  ; Character Input
  (:`Started`
    (`self.Jump`))
  (:`Completed`
    (`self.StopJumping`)))

(event `EnhancedInput|/Game/DemoContent/Blueprint/Input/IA_Shoot`
  (params (ActionValue :type Boolean) (ElapsedSeconds :type "Float (double-precision)") (TriggeredSeconds :type "Float (double-precision)") (InputAction :type "InputAction Object Reference" :default "/Game/DemoContent/Blueprint/Input/IA_Shoot.IA_Shoot"))
  ; Character Input
  (:`Started`
    (`self.OnUseItem`)))

(event `Key|Three`
  (params (Key :type "Key Structure"))
  ; SetBullet
  (:`Pressed`
    (`self.BulletSwitch` 2)))

(event `Key|Four`
  (params (Key :type "Key Structure"))
  ; SetBullet
  (:`Pressed`
    (`self.BulletSwitch` 3)))

(event `Key|Five`
  (params (Key :type "Key Structure"))
  ; SetBullet
  (:`Pressed`
    (`self.BulletSwitch` 4)))

(event `Key|Six`
  (params (Key :type "Key Structure"))
  ; SetBullet
  (:`Pressed`
    (`self.BulletSwitch` 5)))

(fn `BulletSwitch`
  (params (Index :type Integer))
  (bind _output_get (set `self.BulletIndex` Index))
  (`self.BulletSelected` _output_get))

(fn `Spawn Bullet`
  (params (SpawnT :type "Transform Structure (by ref)"))
  (bind (_output_class _output_count _output_cone _output_random) (break `/Game/DemoContent/Blueprint/BulletSpawnInfo` (`|GetArrayItem` (`self.BulletSpawnInfo`) (`self.BulletIndex`))))
  (`BulletFunction.SpawnBulletActor` _output_class SpawnT _output_count _output_cone _output_random self self))

(fn `UpdateLookAtLocation`
  (params (Delta :type "Float (double-precision)"))
  (bind _firstpersoncamera (`self.FirstPersonCamera`))
  (bind _returnvalue (`SceneComponent.K2_GetComponentLocation` _firstpersoncamera))
  (bind (_outhit _returnvalue_2) (`KismetSystemLibrary.LineTraceSingle` _returnvalue (+ _returnvalue (* (`KismetMathLibrary.Conv_RotatorToVector` (`SceneComponent.K2_GetComponentRotation` _firstpersoncamera)) 10000.0)) "TraceTypeQuery1"))
  (bind (_bblockinghit _binitialoverlap _time _distance _location _impactpoint _normal _impactnormal _physmat _hitactor _hitcomponent _hitbonename _bonename _hititem _elementindex _faceindex _tracestart _traceend) (`GameplayStatics.BreakHitResult` _outhit))
  (bind _output_get (set `self.LookAtLocation` (`KismetMathLibrary.SelectVector` _impactpoint _traceend _returnvalue_2)))
  (`SceneComponent.K2_SetWorldLocation` (`self.LookMark`) _output_get false false))

(fn `UserConstructionScript`)